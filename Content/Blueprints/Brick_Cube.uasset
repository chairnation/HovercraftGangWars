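; Brick cube actor that responds to hits by triggering an impact sound, though no sound asset or location appears in the graph.
; Volume comes from the X component of the actor's velocity, expanded to a vector, measured, scaled and clamped to 0–1.
; A DoOnce with a delayed reset limits playback to once every five seconds.
; Every hit also prints that value as debug text, reusing it as the display duration.
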(event `self.ReceiveHit`
  (params (MyComp :type "PrimitiveComponent Object Reference") (Other :type "Actor Object Reference") (OtherComp :type "PrimitiveComponent Object Reference") (bSelfMoved :type Boolean) (HitLocation :type "Vector Structure") (HitNormal :type "Vector Structure") (NormalImpulse :type "Vector Structure") (Hit :type "HitResult Structure (by ref)"))
  (bind _returnvalue (`KismetMathLibrary.FClamp` (/ (`KismetMathLibrary.VSize` (`KismetMathLibrary.Conv_DoubleToVector` (.x (`self.GetVelocity`)))) 50.0)))
  (`KismetSystemLibrary.PrintString` (`KismetStringLibrary.Conv_DoubleToString` _returnvalue) true true (struct :`G` 0.66 :`B` 1.0 :`A` 1.0) _returnvalue)
  (`/Engine/EditorBlueprintResources/StandardMacros.DoOnce` false :!label _label
    (:`Completed`
      (`GameplayStatics.PlaySoundAtLocation` null (0.0 0.0 0.0) (struct) _returnvalue 1.0 0.0 null null null)
      (`KismetSystemLibrary.Delay` 5.0)
      (goto _label :!via `Reset`))))

(fn `UserConstructionScript`)